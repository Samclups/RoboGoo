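; Player character Blueprint, going by its name, that handles HUD setup, NPC-triggered cutscene UI and a score counter, with no movement logic in its graphs.
; It adds the HUD widget on BeginPlay and shows a Cutscene_UI widget when it overlaps a Test_NPC.
; The cutscenemoveon input removes that widget and clears the Cutscene flag.
; A separate IncreaseScore event increments Score by one.
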(event Custom|Increase%20Score
  (Variables|Default|SetScore (+ (Variables|Default|GetScore) 1.0)))

(event EventBeginPlay
  (bind _returnvalue (UserInterface|CreateWidget "/Game/ThirdPersonCPP/Blueprints/HUD.HUD_C"))
  (UserInterface|Viewport|AddtoViewport _returnvalue 0))

(event Collision|EventActorBeginOverlap
  (params (OtherActor :type Actor%20Object%20Reference))
  (Utilities|Casting|CastToTest_NPC OtherActor)
  (bind _returnvalue (UserInterface|CreateWidget "/Game/Jon/Cutscene_UI.Cutscene_UI_C" (Game|GetPlayerController 0)))
  (UserInterface|Viewport|AddtoViewport _returnvalue 0))

(event EventTick
  (params (DeltaSeconds :type Float%20%28single-precision%29)))

(event Input|ActionEvents|InputActioncutscenemoveon
  (params (Key :type Key%20Structure :default "None"))
  (:Pressed
    (Widget|RemovefromParent (stale Collision|EventActorBeginOverlap _returnvalue))
    (Variables|Default|Setcutscene false)))

(fn ConstructionScript)